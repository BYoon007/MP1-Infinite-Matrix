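; BP_TunnelSpawner builds a chain of tunnel segments and populates them with enemies and health packs.
; On BeginPlay it destroys existing tunnels and seeds new ones from the player pawn's location.
; Each new segment attaches at the previous one's SpawnPoint, randomizes its wall and receives a reference to the spawner.
; Random rolls then place either a health pack, one or two enemies, or nothing, offset from the segment's bounds origin along X.
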(event EventBeginPlay
  (CallFunction|SpawnInitialTunnels))

(event Collision|EventActorBeginOverlap
  (params (OtherActor :type Actor%20Object%20Reference)))

(event EventTick
  (params (DeltaSeconds :type Float%20%28single-precision%29)))

(fn ConstructionScript)

(fn SpawnTunnel
  (params (SpawnLocation :type Vector))
  (bind _returnvalue (Game|SpawnActorfromClass "/Game/InfiniteMatrix/Blueprints/BP_Tunnel.BP_Tunnel_C" (Math|Transform|MakeTransform SpawnLocation "0, 0, 0" "1.000000,1.000000,1.000000") "Undefined" "MultiplyWithRoot" 0 0))
  (bind _output_get (Variables|Default|SetNewestTunnel _returnvalue))
  (Variables|/Game/InfiniteMatrix/Blueprints/BP_Tunnel.BP_Tunnel_C|SetTunnelSpawner _output_get self)
  (Default|RandomizeWall _output_get)
  (if (>= (Math|Random|RandomInteger 9) 7)
    (Game|SpawnActorfromClass "/Game/InfiniteMatrix/Blueprints/BP_HealthPack.BP_HealthPack_C" (Math|Transform|MakeTransform (Math|Vector|MakeVector (Math|Random|RandomFloatinRange (+ (.X (Math|Vector|BreakVector (.Origin (Collision|GetActorBounds _output_get false false)))) 1e+02) (+ (.X (Math|Vector|BreakVector (.Origin (Collision|GetActorBounds _output_get false false)))) 8e+02)) (Math|Random|RandomFloatinRange -3e+02 225.0) (Math|Random|RandomFloatinRange -1e+02 2.4e+02)) "0.000000,0.000000,1.000000" "1.000000,1.000000,1.000000") "Undefined" "MultiplyWithRoot" 0 0)
    (elif (>= (Math|Random|RandomInteger 9) 3)
      (Game|SpawnActorfromClass "/Game/InfiniteMatrix/Blueprints/BP_Enemy.BP_Enemy_C" (Math|Transform|MakeTransform (Math|Vector|MakeVector (Math|Random|RandomFloatinRange (+ (.X (Math|Vector|BreakVector (.Origin (Collision|GetActorBounds (Variables|Default|GetNewestTunnel) false false)))) 1e+02) (+ (.X (Math|Vector|BreakVector (.Origin (Collision|GetActorBounds (Variables|Default|GetNewestTunnel) false false)))) 4e+02)) (Math|Random|RandomFloatinRange -9e+01 9e+01) (Math|Random|RandomFloatinRange -1.8e+02 1.4e+02)) "0, 0, 0" "1.000000,1.000000,1.000000") "Undefined" "MultiplyWithRoot" 0 0)
      (if (>= (Math|Random|RandomInteger 9) 7)
        (Game|SpawnActorfromClass "/Game/InfiniteMatrix/Blueprints/BP_Enemy.BP_Enemy_C" (Math|Transform|MakeTransform (Math|Vector|MakeVector (Math|Random|RandomFloatinRange (+ (.X (Math|Vector|BreakVector (.Origin (Collision|GetActorBounds (Variables|Default|GetNewestTunnel) false false)))) 1e+02) (+ (.X (Math|Vector|BreakVector (.Origin (Collision|GetActorBounds (Variables|Default|GetNewestTunnel) false false)))) 4e+02)) (Math|Random|RandomFloatinRange -9e+01 9e+01) (Math|Random|RandomFloatinRange -1.8e+02 1.4e+02)) "0, 0, 0" "1.000000,1.000000,1.000000") "Undefined" "MultiplyWithRoot" 0 0)))))

(fn SpawnTunnelatSpawnPoint
  (CallFunction|SpawnTunnel (Transformation|GetWorldLocation (Variables|/Game/InfiniteMatrix/Blueprints/BP_Tunnel.BP_Tunnel_C|GetSpawnPoint (Variables|Default|GetNewestTunnel)))))

(fn SpawnInitialTunnels
  (Utilities|FlowControl|Sequence
    (:then_0
      (bind _outactors (Actor|GetAllActorsOfClass "/Game/InfiniteMatrix/Blueprints/BP_Tunnel.BP_Tunnel_C"))
      (for _array_element _outactors
        (Actor|DestroyActor _array_element)))
    (:then_1
      (for _index (range 0 2)
        (Utilities|IsValid (Variables|Default|GetNewestTunnel)
          (:Is%20Not%20Valid
            (CallFunction|SpawnTunnel (Transformation|GetActorLocation (Game|Player|GetPlayerPawn 0)))
            (CallFunction|SpawnTunnelatSpawnPoint)))))))